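; BP_BaseRifle is a base rifle actor for a parent pawn, handling projectile firing, ammo and reloads, and destroying itself without a pawn parent.
; Attack spawns a projectile at the muzzle socket if alive, loaded and idle, starts a reset timer and spends ammo.
; An action flag gates firing and reload requests, with dispatchers announcing changes.
; A temporary aim hack points player shots at the HUD's destination, while AI uses base aim rotation.
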(event Custom|OwnerDied
  ;[1 1 1] Comment
  (Variables|Default|SetAlive false))

(event Custom|ReloadAmmo
  (bind _maxammo (Variables|Default|GetMaxAmmo))
  ;[1 1 1] Void Function
  (bind _output_get (Variables|Default|SetCurrentAmmo _maxammo))
  (Default|CallOnAmmoChanged _output_get _maxammo))

(event Custom|RequestReload
  (if (not (Variables|Default|GetActionHappening))
    (Variables|Default|SetActionHappening true)
    (Default|CallOnReloadStart)))

(event EventBeginPlay
  ;[1 1 1] Comment
  (|CallParentFunction)
  (bind _aspawn (Utilities|Casting|CastToPawn (Actor|GetParentActor))
    (:then
      (Variables|Default|SetParentPawn _aspawn)
      (CallFunction|ReloadAmmo))
    (:CastFailed
      (Development|PrintString "The owning actor is not a pawn")
      (Actor|DestroyActor))))

(fn ConstructionScript
  ;[1 1 1] Comment
)

(fn Attack
  (bind _parentpawn (Variables|Default|GetParentPawn))
  ;[1 1 1] Comment
  (if (CallFunction|CanShoot)
    (Game|SpawnActorfromClass (Variables|Default|GetProjectileClass) (Math|Transform|MakeTransform (CallFunction|GetSource) (CallFunction|HACKDONOTCONVERTTOCODE) "1.000000,1.000000,1.000000") "Undefined" "MultiplyWithRoot" (Pawn|GetController _parentpawn) _parentpawn)
    (Variables|Default|SetActionHappening true)
    (Utilities|Time|SetTimerbyEvent (EventDispatchers|CreateEvent :!event ActionStopped) (Variables|Default|GetResetTime))
    (Default|CallOnRifleAttack)
    (CallFunction|UseAmmo)))

(fn CanShoot
  ;[1 1 1] Comment
  (return (Math|Boolean|ANDBoolean (not (Variables|Default|GetActionHappening)) (Variables|Default|GetAlive) (> (Variables|Default|GetCurrentAmmo) 0.0))))

(fn ActionStopped
  ;[1 1 1] Comment
  (Variables|Default|SetActionHappening false)
  (Default|CallOnActionStopped))

(fn GetSource
  ;[1 1 1] Comment
  (return (Transformation|GetSocketLocation (Variables|Default|GetSkeletalMesh) (Variables|Default|GetRifleSocket))))

(fn HACKDONOTCONVERTTOCODE
  ;[1 1 1] Check to see if the player's HUD is the parent pawn to see if you are AI or Player
  (bind _foundwidgets (Widget|GetAllWidgetsOfClass "/Game/Both/WBP_PlayerHUD.WBP_PlayerHUD_C" false))
  (if (== (Class|UserWidget|GetOwningPlayerPawn (Utilities|Array|Get(acopy) _foundwidgets)) (Variables|Default|GetParentPawn))
    (return (Math|Rotator|MakeRotfromX (- (Default|GetDestination (Utilities|Array|Get(acopy) _foundwidgets)) (CallFunction|GetSource))))
    (else
      ;[1 1 1] The AI does the same thing It normally does
      (return (Pawn|GetBaseAimRotation (Variables|Default|GetParentPawn))))))

(fn UseAmmo
  (bind _output_get (Variables|Default|SetCurrentAmmo (Math|Float|Max(Float) (- (Variables|Default|GetCurrentAmmo) 1.0) 0.0)))
  (Default|CallOnAmmoChanged _output_get (Variables|Default|GetMaxAmmo)))