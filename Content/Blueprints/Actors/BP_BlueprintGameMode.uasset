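; Game mode that tracks win and loss by counting enemy characters and showing a results widget.
; On BeginPlay it sorts BP_BaseCharacter actors into player and enemies, binds player-lost and enemy-destroyed events, calls PlayerWin on the player, and creates the widget.
; RemoveEnemy shows the win result and calls PlayerWin when the count reaches zero.
; RemovePlayer shows the widget with UI-only input, but the CurrController assignment it relies on is unconnected.
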(event EventBeginPlay
  (bind _outactors (Actor|GetAllActorsOfClass "/Game/Blueprints/Actors/BP_BaseCharacter.BP_BaseCharacter_C"))
  (for _array_element _outactors
    (bind _asbp_base_player (Utilities|Casting|CastToBP_BasePlayer _array_element)
      (:then
        (EventDispatchers|BindEventtoOnPlayerLost _asbp_base_player (EventDispatchers|CreateEvent :!event RemovePlayer))
        (Variables|Default|SetCurrentPlayer _asbp_base_player)
        (Default|PlayerWin (Variables|Default|GetCurrentPlayer)))
      (:CastFailed
        (CallFunction|AddEnemy _array_element))))
  (bind _returnvalue (Actor|GetActorOfClass (Variables|Default|GetPlayerControllerClass)))
  (bind _returnvalue_2 (UserInterface|CreateWidget (Variables|Default|GetResultsWidgetClass) _returnvalue))
  (Variables|Default|SetResultsWidgetObject _returnvalue_2))

(fn ConstructionScript)

(fn RemoveEnemy
  (params (DestroyedActor :type Actor%20Object%20Reference))
  (bind _resultswidgetobject (Variables|Default|GetResultsWidgetObject))
  (bind _result (Math|Integer|DecrementInt (Variables|Default|GetNumberOfEnemies))
    (:%20%20
      (if (not (> _result 0))
        (UserInterface|Viewport|AddtoViewport _resultswidgetobject 0)
        (Default|SetWin _resultswidgetobject)
        (Default|PlayerWin (Variables|Default|GetCurrentPlayer))))))

(fn AddEnemy
  (params (EnemyActor :type Actor%20Object%20Reference))
  (Game|BindEventtoOnDestroyed EnemyActor (EventDispatchers|CreateEvent :!event RemoveEnemy))
  (Math|Integer|IncrementInt (Variables|Default|GetNumberOfEnemies)))

(fn RemovePlayer
  (bind _resultswidgetobject (Variables|Default|GetResultsWidgetObject))
  (UserInterface|Viewport|AddtoViewport _resultswidgetobject 0)
  (Input|SetInputModeUIOnly (Variables|Default|GetCurrController) _resultswidgetobject "LockAlways" false))