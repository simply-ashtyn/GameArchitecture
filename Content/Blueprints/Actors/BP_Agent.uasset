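; BP_Agent is the AI-controlled combat character: it tints its mesh, fires its weapon and cannot pick up health.
; EnemyAttack and EnemyReload events drive the weapon, and Tick also calls Attack every frame.
; Hurt and death handlers extend the parent to write health ratio to the AI Blackboard, alongside a function that writes current ammo.
; Weapon delegates are bound at BeginPlay, and an "ActionFinished" AI message signals completed actions.
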(event EventBeginPlay
  (bind _weapon (Variables|Default|GetWeapon))
  ;[1 1 1] Comment
  (|CallParentFunction)
  (Rendering|Material|SetVectorParameterValueonMaterials (Variables|Character|GetMesh) (Variables|Default|GetTintName) (Math|Conversions|ToVector(LinearColor) (Variables|Default|GetColor)))
  (EventDispatchers|BindEventtoOnActionStopped (Variables|Default|GetWeapon) (EventDispatchers|CreateEvent :!event HandleActionFinished))
  (CallFunction|UpdateBlackboardHealth 1.0)
  (EventDispatchers|BindEventtoOnAmmoChanged _weapon (EventDispatchers|CreateEvent :!event UpdateBlackboardAmmo))
  (Default|ReloadAmmo _weapon))

(event EventEnemyAttack
  (Default|Attack (Variables|Default|GetWeapon)))

(event EventTick
  (params (DeltaSeconds :type Float%20%28single-precision%29))
  ;[1 1 1] Comment
  (Default|Attack (Variables|Default|GetWeapon)))

(event EventEnemyReload
  (Default|RequestReload (Variables|Default|GetWeapon)))

(fn ConstructionScript
  ;[1 1 1] Comment
  (|CallParentFunction))

(fn HandleActionFinished
  (Class|AIBlueprintHelperLibrary|SendAIMessage self "ActionFinished" 0 true))

(fn UpdateBlackboardHealth
  (params (Ratio :type Float%20%28double-precision%29))
  (AI|Components|Blackboard|SetValueasFloat (AI|GetBlackboard (AI|GetAIController self)) (Variables|Default|GetHealthRatioName) Ratio))

(fn HandleHurt
  (params (Ratio :type Float%20%28double-precision%29))
  (|CallParentFunction Ratio)
  (CallFunction|UpdateBlackboardHealth Ratio))

(fn HandleDeadStart
  (params (Ratio :type Float%20%28double-precision%29))
  (|CallParentFunction Ratio)
  (CallFunction|UpdateBlackboardHealth Ratio))

(fn UpdateBlackboardAmmo
  (params (Current :type Float%20%28double-precision%29) (Max :type Float%20%28double-precision%29))
  (AI|Components|Blackboard|SetValueasFloat (AI|GetBlackboard (AI|GetAIController self)) (Variables|Default|GetAmmoName) Current))

(fn CanPickupHealth
  (return false))