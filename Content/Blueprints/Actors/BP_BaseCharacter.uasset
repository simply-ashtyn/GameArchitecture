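; BP_BaseCharacter is a base character that wires a rifle, health component and animation Blueprint together.
; On BeginPlay it spawns WeaponClass through a child actor component, caches weapon and animation references, and destroys itself if either cast fails.
; Event dispatchers link attack, reload, hurt and death between them; death plays animation, disables collision and notifies the weapon.
; CanPickupHealth returns false by default.
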(event EventBeginPlay
  (bind _childactorcomponent (Variables|Default|GetChildActorComponent))
  ;[1 1 1] Comment
  (|CallParentFunction)
  (ChildActorComponent|SetChildActorClass _childactorcomponent (Variables|Default|GetWeaponClass))
  (bind _asbp_base_rifle (Utilities|Casting|CastToBP_BaseRifle (Variables|/Script/Engine.ChildActorComponent|GetChildActor _childactorcomponent))
    (:then
      (Variables|Default|SetWeapon _asbp_base_rifle)
      (bind _asabp_character_animation (Utilities|Casting|CastToABP_CharacterAnimation (Components|SkeletalMesh|GetAnimInstance (Variables|Character|GetMesh)))
        (:then
          (Variables|Default|SetAnimationBP _asabp_character_animation)
          (EventDispatchers|BindEventtoOnRifleAttack (Variables|Default|GetWeapon) (EventDispatchers|CreateEvent (Variables|Default|GetAnimationBP) :!event FireAnimation))
          ;[1 1 1] Comment
          (EventDispatchers|BindEventtoOnHurt (Variables|Default|GetHealthComponent) (EventDispatchers|CreateEvent :!event HandleHurt))
          (EventDispatchers|BindEventtoOnDeath (Variables|Default|GetHealthComponent) (EventDispatchers|CreateEvent :!event HandleDeadStart))
          (EventDispatchers|BindEventtoOnReloadStart (Variables|Default|GetWeapon) (EventDispatchers|CreateEvent (Variables|Default|GetAnimationBP) :!event ReloadAnimation))
          (EventDispatchers|BindEventtoOnReloadEnded (Variables|Default|GetAnimationBP) (EventDispatchers|CreateEvent (Variables|Default|GetWeapon) :!event ActionStopped))
          (EventDispatchers|BindEventtoOnReloadNow (Variables|Default|GetAnimationBP) (EventDispatchers|CreateEvent (Variables|Default|GetWeapon) :!event ReloadAmmo)))
        (:CastFailed
          (Development|PrintString "We need the correction anation")
          (Actor|DestroyActor))))
    (:CastFailed
      (Development|PrintString "We need a weapon before we can shoot")
      (Actor|DestroyActor))))

(fn ConstructionScript
  ;[1 1 1] Comment
)

(fn HandleHurt
  (params (Ratio :type Float%20%28double-precision%29))
  ;[1 1 1] Comment
  (Default|HitAnimation (Variables|Default|GetAnimationBP) Ratio))

(fn HandleDeadStart
  (params (Ratio :type Float%20%28double-precision%29))
  ;[1 1 1] Comment
  (Default|DeathAnimation (Variables|Default|GetAnimationBP))
  (Collision|SetActorEnableCollision false)
  (Default|OwnerDied (Variables|Default|GetWeapon)))

(fn CanPickupHealth
  (return false))