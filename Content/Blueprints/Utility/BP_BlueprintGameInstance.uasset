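; Game instance that handles level flow, opening levels by index from the GameLevels list and quitting the game.
; Events for main menu (index 0), first level and current level all route through LoadLevelSafe.
; That function validates the index, stores it as the current level and opens the level by name, or prints an error when invalid.
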(event Custom|LoadFirstLevel
  (CallFunction|LoadLevelSafe (Variables|Default|GetFirstLevelIndex)))

(event Custom|QuitGame
  (Game|QuitGame 0 "Quit" false))

(event Custom|LoadCurrentLevel
  (CallFunction|LoadLevelSafe (Variables|Default|GetCurrent%20Level%20Index)))

(event Custom|LoadMainMenu
  (CallFunction|LoadLevelSafe))

(fn LoadLevelSafe
  (params (Level%20Index :type Integer))
  (if (Utilities|Array|IsValidIndex (Variables|Default|GetGameLevels) Level%20Index)
    (Variables|Default|SetCurrent%20Level%20Index Level%20Index)
    (Game|OpenLevel(byName) (Utilities|Array|Get(acopy) (Variables|Default|GetGameLevels) Level%20Index))
    (else
      (Development|PrintString (Utilities|String|Append "Could not load level index " (Utilities|String|ToString(Integer) Level%20Index) ": Invalid index")))))