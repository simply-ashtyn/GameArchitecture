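; AC_HealthComponent is an actor component that tracks health for its owning actor.
; It starts at max health, binds to the owner's OnTakeAnyDamage and clamps health between zero and max on each hit.
; Dispatchers broadcast the health fraction as OnHurt for positive damage or OnHeal otherwise, so negative damage heals.
; At zero health it unbinds from damage and fires OnDeath.
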(event EventBeginPlay
  ;[1 1 1] Comment
  (Variables|Default|SetCurrentHealth (Variables|Default|GetMaxHealth))
  (EventDispatchers|BindEventtoOnTakeAnyDamage (Components|GetOwner) (EventDispatchers|CreateEvent :!event HandleDamage)))

(fn HandleDamage
  (params (DamagedActor :type Actor%20Object%20Reference) (Damage :type Float%20%28single-precision%29) (DamageType :type Damage%20Type%20Object%20Reference) (InstigatedBy :type Controller%20Object%20Reference) (DamageCauser :type Actor%20Object%20Reference))
  ;[1 1 1] Comment
  (bind _output_get (Variables|Default|SetCurrentHealth (Math|Float|Clamp(Float) (- (Variables|Default|GetCurrentHealth) Damage) 0.0 (Variables|Default|GetMaxHealth))))
  (if (> _output_get 0.0)
    (if (> Damage 0.0)
      (Default|CallOnHurt (/ (Variables|Default|GetCurrentHealth) (Variables|Default|GetMaxHealth)))
      (else
        (Default|CallOnHeal (/ (Variables|Default|GetCurrentHealth) (Variables|Default|GetMaxHealth)))))
    (else
      (EventDispatchers|UnbindEventfromOnTakeAnyDamage (Components|GetOwner) (EventDispatchers|CreateEvent :!event HandleDamage))
      (Default|CallOnDeath 0.0))))